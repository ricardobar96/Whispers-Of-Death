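; BP_Weapon is a weapon pickup actor that floats in place until the player interacts with it.
; On BeginPlay, the FloatingAnim timeline moves the Sphere's relative location, then a second timeline plays in reverse and restarts FloatingAnim, forming a continuous bob.
; Interact casts the player character to BP_FirstPersonCharacter, calls its Equip function and destroys the pickup.
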(event EventBeginPlay
  (bind _z_axis_movement (Timeline|FloatingAnim Play)
    (:Update
      (Transformation|SetRelativeLocation (Variables|Default|GetSphere) _z_axis_movement false false))
    (:Finished
      (bind _z_axis_movement_2 (Timeline|Timeline ReverseFromEnd)
        (:Update
          (Transformation|SetRelativeLocation (Variables|Default|GetSphere) _z_axis_movement_2 false false))
        (:Finished
          (Timeline|FloatingAnim PlayFromStart))))))

(event EventInteract
  (bind _asbp_first_person_character (Utilities|Casting|CastToBP_FirstPersonCharacter (Game|GetPlayerCharacter 0)))
  (Default|Equip _asbp_first_person_character)
  (Actor|DestroyActor))

(fn ConstructionScript)